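; BP_TowerGhost is a placement preview tower that shows whether the selected tower can be placed.
; SetGhostTower looks up the row in DT_Towers, applies its mesh to TowerBody and creates a dynamic M_Ghost material instance.
; SetGhostColor tints that instance green or red through its Color parameter, based on CanPlace.
; SelectTarget, separate from the preview logic, picks the first entry in EnemiesInRange as CurrentTarget.
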(fn ConstructionScript)

(fn SelectTarget
  (bind _enemiesinrange (Variables|Default|GetEnemiesInRange))
  (bind _output (Utilities|Array|Get(acopy) _enemiesinrange))
  (if (> (Utilities|Array|Length (Variables|Default|GetEnemiesInRange)) 0)
    (Utilities|IsValid _output
      (:Is%20Valid
        (Variables|Default|SetCurrentTarget _output)))
    (else
      (Variables|Default|SetCurrentTarget 0))))

(fn SetGhostTower
  (params (RowName :type Name))
  (bind _returnvalue (Utilities|GetDataTableRow "/Game/KST/Tower/DT_Towers.DT_Towers" RowName)
    (:then
      (Components|StaticMesh|SetStaticMesh (Variables|Default|GetTowerBody) (.Mesh (Utilities|Struct|BreakS_TowerData _returnvalue)))
      (bind _returnvalue_2 (Rendering|Material|CreateDynamicMaterialInstance (Variables|Default|GetTowerBody) 0 "/Game/KST/Tower/M_Ghost.M_Ghost" "None" :!class /Script/Engine.PrimitiveComponent))
      (bind _output_get (Variables|Default|SetMID _returnvalue_2))
      (Rendering|Material|SetMaterial (Variables|Default|GetTowerBody) 0 _output_get))))

(fn SetGhostColor
  (params (bCanPlace :type Boolean))
  (bind _mid (Variables|Default|GetMID))
  (if bCanPlace
    (Rendering|Material|SetVectorParameterValue _mid "Color" "(R=0.000000,G=1.000000,B=0.000000,A=1.000000)" :!class /Script/Engine.MaterialInstanceDynamic)
    (else
      (Rendering|Material|SetVectorParameterValue _mid "Color" "(R=1.000000,G=0.000000,B=0.000000,A=1.000000)" :!class /Script/Engine.MaterialInstanceDynamic))))
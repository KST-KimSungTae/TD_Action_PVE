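; BP_Tower is a data-driven defense tower that automatically damages enemies within its range.
; On BeginPlay it loads a TowerTable row to set its mesh and range sphere radius, then starts a looping fire timer based on fire rate.
; Range overlaps maintain a BP_Enemy list, and each shot targets the first entry, applying instant damage with a debug line as the only visual.
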(event OnComponentBeginOverlap(RangeCollision)
  (params (OverlappedComponent :type Primitive%20Component%20Object%20Reference) (OtherActor :type Actor%20Object%20Reference) (OtherComp :type Primitive%20Component%20Object%20Reference) (OtherBodyIndex :type Integer) (bFromSweep :type Boolean) (SweepResult :type Hit%20Result%20Structure%20%28by%20ref%29))
  (bind _asbp_enemy (Utilities|Casting|CastToBP_Enemy OtherActor))
  (Utilities|Array|Add (Variables|Default|GetEnemiesInRange) _asbp_enemy))

(event OnComponentEndOverlap(RangeCollision)
  (params (OverlappedComponent :type Primitive%20Component%20Object%20Reference) (OtherActor :type Actor%20Object%20Reference) (OtherComp :type Primitive%20Component%20Object%20Reference) (OtherBodyIndex :type Integer))
  (bind _asbp_enemy (Utilities|Casting|CastToBP_Enemy OtherActor))
  (Utilities|Array|RemoveItem (Variables|Default|GetEnemiesInRange) _asbp_enemy))

(event Custom|FireAtTarget
  (CallFunction|SelectTarget)
  (Utilities|IsValid (Variables|Default|GetCurrentTarget)
    (:Is%20Valid
      (Rendering|Debug|DrawDebugLine (Transformation|GetWorldLocation (Variables|Default|GetTowerBody)) (Transformation|GetWorldLocation (Variables|/Script/Engine.Character|GetMesh (Variables|Default|GetCurrentTarget))) "(R=1.000000,G=0.000000,B=0.945664,A=1.000000)" 0.1 0.0)
      (Game|Damage|ApplyDamage (Variables|Default|GetCurrentTarget) (.Damage (Utilities|Struct|BreakS_TowerData (stale EventBeginPlay _output_get))) 0 self))))

(event EventBeginPlay
  (bind _returnvalue (Utilities|GetDataTableRow (Variables|Default|GetTowerTable) (Variables|Default|GetTowerRowName))
    (:then
      (bind _output_get (Variables|Default|SetStats _returnvalue))
      (Components|StaticMesh|SetStaticMesh (Variables|Default|GetTowerBody) (.Mesh (Utilities|Struct|BreakS_TowerData _output_get)))
      (Components|Sphere|SetSphereRadius (Variables|Default|GetRangeCollision) (.Range (Utilities|Struct|BreakS_TowerData _output_get)) true)
      (Utilities|Time|SetTimerbyEvent (delegate Custom|FireAtTarget) (/ 1.0 (.FireRate (Utilities|Struct|BreakS_TowerData _output_get))) true))))

(fn ConstructionScript)

(fn SelectTarget
  (bind _enemiesinrange (Variables|Default|GetEnemiesInRange))
  (bind _output (Utilities|Array|Get(acopy) _enemiesinrange))
  (if (> (Utilities|Array|Length (Variables|Default|GetEnemiesInRange)) 0)
    (Utilities|IsValid _output
      (:Is%20Valid
        (Variables|Default|SetCurrentTarget _output)))
    (else
      (Variables|Default|SetCurrentTarget 0))))
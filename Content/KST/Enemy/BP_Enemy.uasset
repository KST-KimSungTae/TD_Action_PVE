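; Tower-defense enemy that loads its stats from an EnemyTable row and advances on BP_Core.
; Tick reissues AIMoveTo toward the core, and arrival deals core damage and removes the enemy.
; Damage reduces health, with death paying the player money; both exits decrement the wave manager's alive count, signalling wave clear at zero.
; Overlaps maintain tower, wall and player lists, which this graph never reads, and print debug text.
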(event EventBeginPlay
  (bind _returnvalue (Utilities|GetDataTableRow (Variables|Default|GetEnemyTable) (Variables|Default|GetEnemyRowName))
    (:then
      (bind _output_get (Variables|Default|SetStats _returnvalue))
      (Variables|Default|SetCurrentHealth (* (.MaxHealth (Utilities|Struct|BreakS_EnemyData _output_get)) (Variables|Default|GetHealthMultiplier)))
      (Variables|/Script/Engine.CharacterMovementComponent|SetMaxWalkSpeed (Variables|Character|GetCharacterMovement) (.MoveSpeed (Utilities|Struct|BreakS_EnemyData _output_get)))
      (Transformation|SetActorScale3D (Math|Conversions|ToVector(Float) (.ScaleVisual (Utilities|Struct|BreakS_EnemyData _output_get))))
      (bind _returnvalue_2 (Actor|GetActorOfClass "/Game/KST/Core/BP_Core.BP_Core_C"))
      (Variables|Default|SetTarget _returnvalue_2)
      (Components|Sphere|SetSphereRadius (Variables|Default|GetDetectSphere) (.DetectRange (Utilities|Struct|BreakS_EnemyData (Variables|Default|GetStats))) true))))

(event Collision|EventActorBeginOverlap
  (params (OtherActor :type Actor%20Object%20Reference))
  (bind _asbp_tower (Utilities|Casting|CastToBP_Tower OtherActor)
    (:then
      (Utilities|Array|Add (Variables|Default|GetTowersInRange) _asbp_tower)
      (Development|PrintString "Towerin"))
    (:CastFailed
      (bind _asbp_wall (Utilities|Casting|CastToBp_Wall OtherActor)
        (:then
          (Utilities|Array|Add (Variables|Default|GetWallsInRange) _asbp_wall)
          (Development|PrintString "Wallin"))
        (:CastFailed
          (bind _asbp_top_down_character (Utilities|Casting|CastToBP_TopDownCharacter OtherActor))
          (Utilities|Array|Add (Variables|Default|GetPlayersInRange) _asbp_top_down_character)
          (Development|PrintString "playerin"))))))

(event EventTick
  (params (DeltaSeconds :type Float%20%28single-precision%29))
  (Utilities|IsValid (Variables|Default|GetTarget)
    (:Is%20Valid
      (AI|AIMoveTo self (Transformation|GetActorLocation (Variables|Default|GetTarget)) 0 (Components|Capsule|GetScaledCapsuleRadius (Variables|/Game/KST/Core/BP_Core.BP_Core_C|GetCapsule (stale EventBeginPlay _returnvalue_2))) false
        (:OnSuccess
          (bind _asbp_core (Utilities|Casting|CastToBP_Core (Variables|Default|GetTarget)))
          (Default|TakeCoreDamage _asbp_core (.CoreDamage (Utilities|Struct|BreakS_EnemyData (Variables|Default|GetStats))))
          (CallFunction|NotifyDeath)
          (Actor|DestroyActor))))))

(event Game|Damage|EventAnyDamage
  (params (Damage :type Float%20%28single-precision%29) (DamageType :type Damage%20Type%20Object%20Reference) (InstigatedBy :type Controller%20Object%20Reference) (DamageCauser :type Actor%20Object%20Reference))
  (bind _output_get (Variables|Default|SetCurrentHealth (- (Variables|Default|GetCurrentHealth) Damage)))
  (Development|PrintString (Utilities|String|ToString(Float) _output_get))
  (if (<= _output_get 0.0)
    (bind _asbp_top_down_character (Utilities|Casting|CastToBP_TopDownCharacter (Game|GetPlayerCharacter 0)))
    (Variables|/Game/TopDown/Blueprints/BP_TopDownCharacter.BP_TopDownCharacter_C|SetMoney _asbp_top_down_character (+ (Variables|/Game/TopDown/Blueprints/BP_TopDownCharacter.BP_TopDownCharacter_C|GetMoney _asbp_top_down_character) (.MoneyReward (Utilities|Struct|BreakS_EnemyData (Variables|Default|GetStats)))))
    (CallFunction|NotifyDeath)
    (Actor|DestroyActor)))

(event Collision|EventActorEndOverlap
  (params (OtherActor :type Actor%20Object%20Reference))
  (bind _asbp_tower (Utilities|Casting|CastToBP_Tower OtherActor)
    (:then
      (Utilities|Array|RemoveItem (Variables|Default|GetTowersInRange) _asbp_tower)
      (Development|PrintString "Towerout"))
    (:CastFailed
      (bind _asbp_wall (Utilities|Casting|CastToBp_Wall OtherActor)
        (:then
          (Utilities|Array|RemoveItem (Variables|Default|GetWallsInRange) _asbp_wall)
          (Development|PrintString "Wallout"))
        (:CastFailed
          (bind _asbp_top_down_character (Utilities|Casting|CastToBP_TopDownCharacter OtherActor))
          (Utilities|Array|RemoveItem (Variables|Default|GetPlayersInRange) _asbp_top_down_character)
          (Development|PrintString "playerout"))))))

(fn ConstructionScript)

(fn NotifyDeath
  (bind _returnvalue (Actor|GetActorOfClass "/Game/KST/Enemy/BP_WaveMananger.BP_WaveMananger_C"))
  (bind _output_get (Variables|/Game/KST/Enemy/BP_WaveMananger.BP_WaveMananger_C|SetEnemiesAlive _returnvalue (- (Variables|/Game/KST/Enemy/BP_WaveMananger.BP_WaveMananger_C|GetEnemiesAlive _returnvalue) 1)))
  (if (<= _output_get 0)
    (Default|OnWaveCleared _returnvalue)))
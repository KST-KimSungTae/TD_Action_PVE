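; Grunt enemy for a wave-based core defense mode that walks to BP_Core, deals fixed damage on arrival and destroys itself.
; It finds the core on BeginPlay and reissues AI MoveTo every Tick, using the core's capsule radius as acceptance distance.
; Incoming damage reduces Health, and death awards Money to the player's BP_TopDownCharacter.
; Both endings call NotifyDeath, which decrements BP_WaveMananger's EnemiesAlive and triggers OnWaveCleared at zero.
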(event EventBeginPlay
  (bind _returnvalue (Actor|GetActorOfClass "/Game/KST/Core/BP_Core.BP_Core_C"))
  (Variables|Default|SetTarget _returnvalue))

(event Collision|EventActorBeginOverlap
  (params (OtherActor :type Actor%20Object%20Reference)))

(event EventTick
  (params (DeltaSeconds :type Float%20%28single-precision%29))
  (Utilities|IsValid (Variables|Default|GetTarget)
    (:Is%20Valid
      (AI|AIMoveTo self (Transformation|GetActorLocation (Variables|Default|GetTarget)) 0 (Components|Capsule|GetScaledCapsuleRadius (Variables|/Game/KST/Core/BP_Core.BP_Core_C|GetCapsule (stale EventBeginPlay _returnvalue))) false
        (:OnSuccess
          (bind _asbp_core (Utilities|Casting|CastToBP_Core (Variables|Default|GetTarget)))
          (Default|TakeCoreDamage _asbp_core 1e+01)
          (CallFunction|NotifyDeath)
          (Development|PrintString (Utilities|String|ToString(Float) (Variables|/Game/KST/Core/BP_Core.BP_Core_C|GetCoreHealth _asbp_core)))
          (Actor|DestroyActor))))))

(event Game|Damage|EventAnyDamage
  (params (Damage :type Float%20%28single-precision%29) (DamageType :type Damage%20Type%20Object%20Reference) (InstigatedBy :type Controller%20Object%20Reference) (DamageCauser :type Actor%20Object%20Reference))
  (bind _output_get (Variables|Default|SetHealth (- (Variables|Default|GetHealth) Damage)))
  (Development|PrintString (Utilities|String|ToString(Float) (Variables|Default|GetHealth)))
  (if (<= _output_get 0.0)
    (bind _asbp_top_down_character (Utilities|Casting|CastToBP_TopDownCharacter (Game|GetPlayerCharacter 0)))
    (bind _output_get_2 (Variables|/Game/TopDown/Blueprints/BP_TopDownCharacter.BP_TopDownCharacter_C|SetMoney _asbp_top_down_character (+ (Variables|/Game/TopDown/Blueprints/BP_TopDownCharacter.BP_TopDownCharacter_C|GetMoney _asbp_top_down_character) 10)))
    (Development|PrintString (Utilities|String|ToString(Integer) _output_get_2))
    (CallFunction|NotifyDeath)
    (Actor|DestroyActor)))

(fn ConstructionScript)

(fn NotifyDeath
  (bind _returnvalue (Actor|GetActorOfClass "/Game/KST/Enemy/BP_WaveMananger.BP_WaveMananger_C"))
  (bind _output_get (Variables|/Game/KST/Enemy/BP_WaveMananger.BP_WaveMananger_C|SetEnemiesAlive _returnvalue (- (Variables|/Game/KST/Enemy/BP_WaveMananger.BP_WaveMananger_C|GetEnemiesAlive _returnvalue) 1)))
  (if (<= _output_get 0)
    (Default|OnWaveCleared _returnvalue)))
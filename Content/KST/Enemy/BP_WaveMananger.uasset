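; Wave manager that tracks the current wave number and game state across wave start, wave clear and game over.
; StartWave advances the wave, computes a linearly growing enemy count and passes it to the BP_Spawner found in the level.
; OnWaveCleared switches state and, like StartWave, prints debug messages.
; GameOver sets its state, shows the WBP_GameOver widget and pauses the game.
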(event Custom|StartWave
  (Variables|Default|SetCurrentWave (+ (Variables|Default|GetCurrentWave) 1))
  (Variables|Default|SetCurrentState "NewEnumerator1")
  (bind _output_get (Variables|Default|SetEnemiesAlive (+ (Variables|Default|GetBaseEnemies) (* (- (Variables|Default|GetCurrentWave) 1) (Variables|Default|GetEnemiesPerWaveIncrement)))))
  (bind _returnvalue (Actor|GetActorOfClass "/Game/KST/Enemy/BP_Spawner.BP_Spawner_C"))
  (Default|StartSpawning _returnvalue _output_get)
  (Development|PrintString "Wave ")
  (Development|PrintString (Utilities|String|ToString(Integer) (Variables|Default|GetCurrentWave)))
  (Development|PrintString "Start"))

(event Custom|OnWaveCleared
  (Variables|Default|SetCurrentState "NewEnumerator0")
  (Development|PrintString "Wave ")
  (Development|PrintString (Utilities|String|ToString(Integer) (Variables|Default|GetCurrentWave)))
  (Development|PrintString "클리어"))

(event Custom|GameOver
  (Variables|Default|SetCurrentState "NewEnumerator2")
  (bind _returnvalue (UserInterface|CreateWidget "/Game/KST/UI/WBP_GameOver.WBP_GameOver_C" (Game|GetPlayerController 0)))
  (UserInterface|Viewport|AddtoViewport _returnvalue 0)
  (Game|SetGamePaused (Utilities|Enum|Equal(Enum) (Variables|Default|GetCurrentState) "NewEnumerator2")))

(fn ConstructionScript)
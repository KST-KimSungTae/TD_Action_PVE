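; BP_Spawner is an enemy spawner that produces a requested number of BP_Enemy actors at its own transform.
; StartSpawning stores the count, resets the tally and starts a looping timer at SpawnInterval, so the first enemy appears after one interval.
; Each SpawnOne tick spawns an enemy, adjusting for collisions but always spawning, and clears the timer once the count is reached.
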(event Custom|SpawnOne
  (Game|SpawnActorfromClass "/Game/KST/Enemy/BP_Enemy.BP_Enemy_C" (Transformation|GetActorTransform) "AdjustIfPossibleButAlwaysSpawn" "MultiplyWithRoot" 0 0)
  (Variables|Default|SetSpawned (+ (Variables|Default|GetSpawned) 1))
  (if (>= (Variables|Default|GetSpawned) (Variables|Default|GetNumToSpawn))
    (Utilities|Time|ClearandInvalidateTimerbyHandle (stale Custom|StartSpawning _returnvalue))))

(event Custom|StartSpawning
  (params (Count :type Integer))
  (Variables|Default|SetNumToSpawn Count)
  (Variables|Default|SetSpawned 0)
  (bind _returnvalue (Utilities|Time|SetTimerbyEvent (delegate Custom|SpawnOne) (Variables|Default|GetSpawnInterval) true)))

(event EventBeginPlay)

(fn ConstructionScript)